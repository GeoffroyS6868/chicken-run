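; BP_Wolf is an AI wolf enemy that chases the player and knocks them into the air on contact.
; A PawnSensing sighting sets a seeing flag, never cleared here, and calls FollowPlayer, which issues an AI move toward player zero.
; When its capsule hits a BP_Character, it launches that character along the wolf mesh's forward vector, scaled by PushForce, with a fixed upward boost.
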(event `self.PawnSensing.OnSeePawn`
  (params (Pawn :type "Pawn Object Reference"))
  (set `self.IsSeeingPlayer` true)
  (`self.FollowPlayer`))

(event `FollowPlayer`
  (if (`self.IsSeeingPlayer`)
    (`|AIMoveTo` self (0.0 0.0 0.0) (`GameplayStatics.GetPlayerCharacter` 0))))

(event `self.CapsuleComponent.OnComponentHit`
  (params (HitComponent :type "PrimitiveComponent Object Reference") (OtherActor :type "Actor Object Reference") (OtherComp :type "PrimitiveComponent Object Reference") (NormalImpulse :type "Vector Structure") (Hit :type "HitResult Structure (by ref)"))
  (bind _pushforce (`self.PushForce`))
  (bind (_returnvalue_x _returnvalue_y) (`KismetMathLibrary.BreakVector` (`SceneComponent.GetForwardVector` (`self.Mesh`))))
  (bind _asbp_character (cast `/Game/Blueprints/Character/BP_Character` OtherActor))
  (`self.LaunchCharacter` _asbp_character (`KismetMathLibrary.MakeVector` (* _pushforce _returnvalue_x) (* _pushforce _returnvalue_y) 1000.0) false false))

(fn `UserConstructionScript`)