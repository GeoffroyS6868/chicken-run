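; BP_Checkpoint is a checkpoint actor that updates the player's respawn point when a BP_Character first enters its trigger zone.
; The respawn location comes from a skeletal mesh, hidden at BeginPlay, and a flag guards against repeat activation.
; Activation plays a sound and runs two chained timelines that shrink the red flag, then show and grow the green one, before deactivating the trigger component.
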(event `self.ReceiveBeginPlay`
  (`SceneComponent.SetVisibility` (`self.SkeletalMesh`) false false))

(event `self.C_TriggerZone.OnComponentBeginOverlap`
  (params (OverlappedComponent :type "PrimitiveComponent Object Reference") (OtherActor :type "Actor Object Reference") (OtherComp :type "PrimitiveComponent Object Reference") (OtherBodyIndex :type Integer) (bFromSweep :type Boolean) (SweepResult :type "HitResult Structure (by ref)"))
  (bind _sm_flagred (`self.SM_FlagRed`))
  ;[1 1 1] Character Trigger
  (if (not (`self.IsActivated`))
    (bind _asbp_character (cast `/Game/Blueprints/Character/BP_Character` OtherActor))
    (`/Game/Blueprints/Character/BP_Character.SetNewRespawnPoint` _asbp_character (`SceneComponent.K2_GetComponentLocation` (`self.SkeletalMesh`)))
    (set `self.IsActivated` true)
    (`GameplayStatics.PlaySoundAtLocation` "/Game/Audio/SOUND_Checkpoint.SOUND_Checkpoint" (`SceneComponent.K2_GetComponentLocation` (`self.SM_FlagGreen`)) (struct) 1.0 1.0 0.0 null null null null)
    (bind (_direction _shrink) (`Timeline|Timeline`)
      (:`Update`
        (`SceneComponent.SetRelativeScale3D` _sm_flagred (`KismetMathLibrary.MakeVector` _shrink _shrink _shrink)))
      (:`Finished`
        (`ActorComponent.Deactivate` _sm_flagred)
        (`SceneComponent.SetVisibility` (`self.SM_FlagGreen`) true false)
        (bind (_direction_2 _growth) (`Timeline|Timeline_0`)
          (:`Update`
            (`SceneComponent.SetRelativeScale3D` (`self.SM_FlagGreen`) (`KismetMathLibrary.MakeVector` _growth _growth _growth)))
          (:`Finished`
            (`ActorComponent.Deactivate` (`self.C_TriggerZone`))))))))

(fn `UserConstructionScript`)