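; BP_Magnet is an interactable magnet actor that triggers movement of a matching island magnet.
; On Interact, it stores its Magnet component's world location in PositionToGo, then searches all BP_IslandMagnet actors.
; The first whose MagnetValue is one higher than its own receives a MoveMagnet call, so magnets pair by sequential value.
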(event `/Game/Blueprints/Core/BPI_Interact.Interact`
  (params (Player :type "Character Object Reference"))
  ;[1 1 1] Interact
  (set `self.PositionToGo` (`SceneComponent.K2_GetComponentLocation` (`self.Magnet`)))
  (bind _outactors (`GameplayStatics.GetAllActorsOfClass` "/Game/Blueprints/Actor/BP_IslandMagnet.BP_IslandMagnet_C"))
  (for _array_element _outactors
    (if (== (`/Game/Blueprints/Actor/BP_IslandMagnet.MagnetValue` _array_element) (+ (`self.MagnetValue`) 1))
      (`/Game/Blueprints/Actor/BP_IslandMagnet.MoveMagnet` _array_element)
      (break))))

(fn `UserConstructionScript`)