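; BP_Gate is a level-select gate actor that sends the game to the level matching its TriggerBoxType enum.
; The construction script labels its text render with the one-based level number.
; IsActivated asks BP_GameInstance whether that level is available, gating both Portal activation at BeginPlay and the trigger box overlap.
; An overlap on an available gate stores the enum name as the game instance's LevelName, then opens LoadingScreen.
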(event `self.ReceiveBeginPlay`
  (bind _activated (`self.IsActivated`))
  (if _activated
    (`ActorComponent.Activate` (`self.Portal`) false)))

(event `self.Box.OnComponentBeginOverlap`
  (params (OverlappedComponent :type "PrimitiveComponent Object Reference") (OtherActor :type "Actor Object Reference") (OtherComp :type "PrimitiveComponent Object Reference") (OtherBodyIndex :type Integer) (bFromSweep :type Boolean) (SweepResult :type "HitResult Structure (by ref)"))
  (bind _activated (`self.IsActivated`))
  (if _activated
    (bind _asbp_game_instance (cast `/Game/Blueprints/Core/BP_GameInstance` (`GameplayStatics.GetGameInstance`)))
    (set `/Game/Blueprints/Core/BP_GameInstance.LevelName` (`KismetStringLibrary.Conv_StringToName` (`|GetEnumeratorNameAsString` (`self.TriggerBoxType`))) _asbp_game_instance)
    (`GameplayStatics.OpenLevel` "LoadingScreen" false)))

(fn `IsActivated`
  (returns (Activated :type Boolean))
  (bind _asbp_game_instance (cast `/Game/Blueprints/Core/BP_GameInstance` (`GameplayStatics.GetGameInstance`)))
  (bind _isavailable (`/Game/Blueprints/Core/BP_GameInstance.IsLevelAvailable` _asbp_game_instance (`KismetMathLibrary.Conv_ByteToInt` (`self.TriggerBoxType`))))
  (return _isavailable))

(fn `UserConstructionScript`
  (bind _result (`/Engine/EditorBlueprintResources/StandardMacros.IncrementInt` (`KismetMathLibrary.Conv_ByteToInt` (`self.TriggerBoxType`)))
    (:`  `
      (`TextRenderComponent.K2_SetText` (`self.TextRender`) (`KismetTextLibrary.Conv_StringToText` (`KismetStringLibrary.Concat_StrStr` "Level " (`KismetStringLibrary.Conv_IntToString` _result)))))))