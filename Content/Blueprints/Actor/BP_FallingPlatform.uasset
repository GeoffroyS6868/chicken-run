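; A falling platform actor that drops after the player steps on it and later resets to its starting position.
; When the player character overlaps the Box, a short delay precedes enabling physics simulation on SMPlatform.
; After a further delay, physics turns off and the mesh teleports to the actor location and rotation saved at BeginPlay, using the mesh's saved world scale.
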(event `self.ReceiveBeginPlay`
  (set `self.InitTransform` (`self.GetTransform`))
  (set `self.InitScale` (`SceneComponent.K2_GetComponentScale` (`self.SM_Platform`))))

(event `self.Box.OnComponentBeginOverlap`
  (params (OverlappedComponent :type "PrimitiveComponent Object Reference") (OtherActor :type "Actor Object Reference") (OtherComp :type "PrimitiveComponent Object Reference") (OtherBodyIndex :type Integer) (bFromSweep :type Boolean) (SweepResult :type "HitResult Structure (by ref)"))
  (if (== OtherActor (`GameplayStatics.GetPlayerCharacter` 0))
    (`KismetSystemLibrary.Delay` 1.0)
    (`PrimitiveComponent.SetSimulatePhysics` (`self.SM_Platform`) true)
    (`KismetSystemLibrary.Delay` 5.0)
    (`PrimitiveComponent.SetSimulatePhysics` (`self.SM_Platform`) false)
    (`SceneComponent.K2_SetWorldTransform` (`self.SM_Platform`) (`KismetMathLibrary.MakeTransform` (.location (`self.InitTransform`)) (.rotation (`self.InitTransform`)) (`self.InitScale`)) false true)))

(fn `UserConstructionScript`)